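; BP_OutLine drives SDF-based face shading on the March character mesh from a directional light's yaw.
; The construction script swaps the face material for a dynamic instance and starts a fast looping timer, apparently for Update.
; Update uses dot and cross products of light and head-socket forward vectors to encode signed light direction.
; A curve remaps that value into the material's SDF_Location parameter.
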(event Custom|Update
  (bind _directionlight (Variables|Default|GetDirectionLight))
  (bind _sk_march (Variables|Default|GetSK_March))
  (bind _returnvalue (Transformation|GetSocketRotation _sk_march "頭"))
  (bind _returnvalue_2 (Transformation|GetActorRotation _directionlight))
  (bind _returnvalue_3 (Math|Rotator|MakeRotator 0.0 0.0 (.yaw _returnvalue_2)))
  (bind _returnvalue_4 (Math|Vector|GetForwardVector _returnvalue))
  (bind _returnvalue_5 (Math|Vector|GetForwardVector _returnvalue_3))
  (bind _returnvalue_6 (Math|Vector|DotProduct _returnvalue_5 _returnvalue_4))
  (bind _returnvalue_7 (/ _returnvalue_6 2.0))
  (Utilities|IsValid _directionlight
    (:Is%20Valid
      (if (<= (.z (Math|Vector|CrossProduct _returnvalue_5 _returnvalue_4)) 0.0)
        (if (<= _returnvalue_6 0.0)
          (Variables|Default|SetSDF_Location (+ _returnvalue_7 1.0))
          (else
            (Variables|Default|SetSDF_Location (- _returnvalue_7 1.0))))
        (else
          (Variables|Default|SetSDF_Location (/ _returnvalue_6 -2.0))))
      ;[1 1 1] 背对着是-1，正对着是1，脸的右侧是-0.5，左侧是0.5
      (Rendering|Material|SetScalarParameterValue (Variables|Default|GetFace) "SDF_Location" (Math|Curves|GetFloatValue (Variables|Default|GetSDF_Curve) (Variables|Default|GetSDF_Location)) :!class /Script/Engine.MaterialInstanceDynamic))))

(fn ConstructionScript
  (bind _facematerial (Variables|Default|GetFaceMaterial))
  (Utilities|FlowControl|Sequence
    (:then_0
      (bind _returnvalue (Rendering|Material|CreateDynamicMaterialInstance _facematerial "None" "None" :!class /Script/Engine.KismetMaterialLibrary))
      (bind _output_get (Variables|Default|SetFace _returnvalue))
      (Rendering|Material|SetMaterial (Variables|Default|GetSK_March) (Utilities|Array|FindItem (Rendering|Material|GetMaterials (Variables|Default|GetSK_March)) _facematerial) _output_get))
    (:then_1
      (Utilities|Time|SetTimerbyEvent (EventDispatchers|CreateEvent :!event Custom|Update) 0.01 true))))